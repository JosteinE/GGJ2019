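; Lid is an interactable prop that swings open when the player has a key.
; Interact checks UnlockedKey on the ThirdPersonCharacter, then sets a -90 degree target rotation, flags LidOpen and consumes the key.
; Tick eases PivotPoint toward that target with a fixed-alpha rotator lerp, so its speed depends on frame rate.
; The closing logic is unconnected, so nothing here shuts the lid again.
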(event EventBeginPlay)

(event Collision|EventActorBeginOverlap
  (params (OtherActor :type Actor%20Object%20Reference)))

(event EventTick
  (params (DeltaSeconds :type Float%20%28single-precision%29))
  (bind _pivotpoint (Variables|Default|GetPivotPoint))
  (Transformation|SetRelativeRotation _pivotpoint (Math|Rotator|Lerp(Rotator) (Variables|/Script/Engine.SceneComponent|GetRelativeRotation _pivotpoint) (Variables|Default|GetrotateRate) 0.2) false false))

(event EventInteract
  (bind _asthird_person_character (Utilities|Casting|CastToThirdPersonCharacter (Game|GetPlayerCharacter 0)))
  (if (Variables|/Script/GGJ2019.GGJ2019Character|GetbUnlockedKey _asthird_person_character)
    (Variables|Default|SetrotateRate "0,0.000000,-90.000000")
    (Variables|Default|SetlidOpen true)
    (bind _asthird_person_character_2 (Utilities|Casting|CastToThirdPersonCharacter (Game|GetPlayerCharacter 0)))
    (Variables|/Script/GGJ2019.GGJ2019Character|SetbUnlockedKey _asthird_person_character_2 false)))

(fn ConstructionScript)