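; Evil_Spike is a hazard prop that alters the player's health after the player character overlaps it.
; Tick compares the OtherActor output of the otherwise unwired BeginOverlap event to player 0's character, with no end-overlap handling.
; On a match, while ThirdPersonCharacter's PlayerHealth is above zero, it overwrites that health with SpikeDamage scaled by DeltaSeconds rather than subtracting it.
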(event EventBeginPlay)

(event Collision|EventActorBeginOverlap
  (params (OtherActor :type Actor%20Object%20Reference)))

(event EventTick
  (params (DeltaSeconds :type Float%20%28single-precision%29))
  (bind _returnvalue (Game|GetPlayerCharacter 0))
  (if (== (stale Collision|EventActorBeginOverlap OtherActor) _returnvalue)
    (bind _asthird_person_character (Utilities|Casting|CastToThirdPersonCharacter _returnvalue))
    (if (> (Variables|/Script/GGJ2019.GGJ2019Character|GetplayerHealth _asthird_person_character) 0.0)
      (Variables|/Script/GGJ2019.GGJ2019Character|SetplayerHealth _asthird_person_character (* (Variables|Default|GetSpikeDamage) DeltaSeconds)))))

(fn ConstructionScript)