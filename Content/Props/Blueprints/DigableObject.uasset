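; DigableObject is a prop that shrinks while the player digs at it with a spade.
; Each Tick it loops over overlapping ThirdPersonCharacter actors, then checks player 0's character for the UsingSpade and SwingingCurrent states.
; When both hold, it subtracts delta time plus a fixed step from its scale, so shrink speed depends on frame rate.
; The graph has no lower scale limit or destroy step.
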(event EventBeginPlay)

(event Collision|EventActorBeginOverlap
  (params (OtherActor :type Actor%20Object%20Reference)))

(event EventTick
  (params (DeltaSeconds :type Float%20%28single-precision%29))
  (for _array_element (Collision|GetOverlappingActors "/Game/ThirdPersonCPP/Blueprints/ThirdPersonCharacter.ThirdPersonCharacter_C" :!class /Script/Engine.Actor)
    (bind _asthird_person_character (Utilities|Casting|CastToThirdPersonCharacter (Game|GetPlayerCharacter 0)))
    (if (and (Variables|/Script/GGJ2019.GGJ2019Character|GetbUsingSpade _asthird_person_character) (Variables|/Script/GGJ2019.GGJ2019Character|GetbSwingingCurrent _asthird_person_character))
      (Transformation|SetActorScale3D (- (- (Transformation|GetActorScale3D) DeltaSeconds) 0.05)))))

(fn ConstructionScript)