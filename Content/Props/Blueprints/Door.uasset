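; Interactive door prop that swings open and closed around a pivot component.
; The Interact event toggles the DoorOpen flag and switches RotateRate, used as a target rotation, between closed and a 90-degree open pose.
; Tick lerps the PivotPoint's relative rotation toward that target with a fixed alpha every frame, giving an eased but frame-rate-dependent swing.
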(event EventBeginPlay)

(event Collision|EventActorBeginOverlap
  (params (OtherActor :type Actor%20Object%20Reference)))

(event EventTick
  (params (DeltaSeconds :type Float%20%28single-precision%29))
  (bind _pivotpoint (Variables|Default|GetPivotPoint))
  (Transformation|SetRelativeRotation _pivotpoint (Math|Rotator|Lerp(Rotator) (Variables|/Script/Engine.SceneComponent|GetRelativeRotation _pivotpoint) (Variables|Default|GetrotateRate) 0.2) false false))

(event EventInteract
  (if (Variables|Default|GetdoorOpen)
    (Variables|Default|SetrotateRate "0, 0, 0")
    (Variables|Default|SetdoorOpen false)
    (else
      (Variables|Default|SetrotateRate "0,90.000000, 0")
      (Variables|Default|SetdoorOpen true))))

(fn ConstructionScript)