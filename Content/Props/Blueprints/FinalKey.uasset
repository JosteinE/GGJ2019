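; Interactable final key pickup prop that records the key as unlocked on the player's ThirdPersonCharacter.
; On Interact, it sets UnlockedFinalKey only if the actor's object name is exactly "FinalKey", so the unlock depends on instance naming.
; Regardless of that check, it then destroys itself and adds a newly created InventoryHUD widget to the viewport, provided the character cast succeeds.
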(event EventInteract
  (bind _asthird_person_character (Utilities|Casting|CastToThirdPersonCharacter (Game|GetPlayerCharacter 0)))
  (if (Utilities|Enum|Equal(Enum) (Utilities|GetObjectName self) "FinalKey")
    (Variables|/Game/ThirdPersonCPP/Blueprints/ThirdPersonCharacter.ThirdPersonCharacter_C|SetbUnlockedFinalKey _asthird_person_character true))
  (Actor|DestroyActor)
  (bind _returnvalue (UserInterface|CreateWidget "/Game/ThirdPersonCPP/Blueprints/HUD/InventoryHUD.InventoryHUD_C" (Game|GetPlayerController 0)))
  (UserInterface|Viewport|AddtoViewport _returnvalue 0))

(fn ConstructionScript)