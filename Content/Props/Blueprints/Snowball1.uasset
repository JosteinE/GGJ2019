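; Snowball prop that grows as it moves and destroys itself when its scale reaches 2 on all axes.
; Each Tick, while speed is above a small threshold, it adds a fixed scale step, so growth depends on frame rate.
; The same step sets the Snowball component's mass scale to its current mass plus one, feeding mass back into the multiplier.
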(event EventTick
  (params (DeltaSeconds :type Float%20%28single-precision%29))
  (bind _returnvalue (Transformation|GetActorScale3D))
  (bind _snowball (Variables|Default|GetSnowball))
  (if (Math|Vector|Equal(Vector) _returnvalue "2.000000,2.000000,2.000000" 0.0001)
    (Actor|DestroyActor)
    (elif (> (Math|Vector|VectorLength (Transformation|GetVelocity)) 5.0)
      (Transformation|SetActorScale3D (+ _returnvalue 0.001))
      (Class|PrimitiveComponent|SetMassScale _snowball "None" (+ (Physics|GetMass _snowball) 1.0)))))

(fn ConstructionScript)