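; Readable book prop that shows note text in a dialogue widget, one line per interaction.
; On BeginPlay it caches the dialogue data table rows matching its NOTEID.
; Each Interact increments the line counter and looks up the row matching ConversationID and LineID.
; The widget closes and the counter resets when no single line matches or the ThirdPersonCharacter leaves the box.
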(event OnComponentEndOverlap(Box)
  (params (OverlappedComponent :type Primitive%20Component%20Object%20Reference) (OtherActor :type Actor%20Object%20Reference) (OtherComp :type Primitive%20Component%20Object%20Reference) (OtherBodyIndex :type Integer))
  (Utilities|Casting|CastToThirdPersonCharacter OtherActor)
  (Utilities|IsValid (Variables|Default|GetDialogueWidget)
    (:Is%20Valid
      (Widget|RemovefromParent (Variables|Default|GetDialogueWidget))
      (Variables|Default|SetDialogueWidget 0)
      (Variables|Default|SetLineCurrnet 0))))

(event EventBeginPlay
  (bind _outrownames (DataTable|GetDataTableRowNames "/Game/ThirdPersonCPP/Blueprints/HUD/Dialogue/GGJ2019Dialogue_Take5.GGJ2019Dialogue_Take5"))
  (for _array_element _outrownames
    (bind _returnvalue (Utilities|GetDataTableRow "/Game/ThirdPersonCPP/Blueprints/HUD/Dialogue/GGJ2019Dialogue_Take5.GGJ2019Dialogue_Take5" _array_element)
      (:then
        (if (== (.NOTE_ID (Utilities|Struct|BreakDialogueStructure _returnvalue)) (Variables|Default|GetNOTE_ID))
          (Utilities|Array|Add (Variables|Default|GetMyDialogue) _array_element))))))

(event EventInteract
  (Math|Integer|IncrementInt (Variables|Default|GetLineCurrnet)
    (:%20%20
      (CallFunction|DialogueCreate))))

(fn ConstructionScript)

(fn DialogueCreate
  (Utilities|IsValid (Variables|Default|GetDialogueWidget)
    (:Is%20Valid
      (bind _returnedline (CallFunction|DialogueGetLine))
      (if (Utilities|Enum|NotEqual(Enum) (Variables|Default|GetEmptyText) _returnedline)
        (Variables|/Game/ThirdPersonCPP/Blueprints/HUD/Dialogue/DialogueWidget.DialogueWidget_C|SetDialogueText (Variables|Default|GetDialogueWidget) _returnedline)))
    (:Is%20Not%20Valid
      (bind _returnvalue (UserInterface|CreateWidget "/Game/ThirdPersonCPP/Blueprints/HUD/Dialogue/DialogueWidget.DialogueWidget_C" (Game|GetPlayerController 0)))
      (bind _output_get (Variables|Default|SetDialogueWidget _returnvalue))
      (UserInterface|Viewport|AddtoViewport _output_get 0)
      (bind _returnedline_2 (CallFunction|DialogueGetLine))
      (Variables|/Game/ThirdPersonCPP/Blueprints/HUD/Dialogue/DialogueWidget.DialogueWidget_C|SetDialogueText (Variables|Default|GetDialogueWidget) _returnedline_2))))

(fn DialogueGetLine
  (for _array_element (Variables|Default|GetMyDialogue)
    (bind _returnvalue (Utilities|GetDataTableRow "/Game/ThirdPersonCPP/Blueprints/HUD/Dialogue/GGJ2019Dialogue_Take5.GGJ2019Dialogue_Take5" _array_element)
      (:then
        (if (and (== (.Conversation_ID (Utilities|Struct|BreakDialogueStructure _returnvalue)) (Variables|Default|GetConversation_ID)) (== (.Line_ID (Utilities|Struct|BreakDialogueStructure _returnvalue)) (Variables|Default|GetLineCurrnet)))
          (Utilities|Array|Add (LocalVariables|GetReturnedLines) (.Dialogue (Utilities|Struct|BreakDialogueStructure _returnvalue)))))))
  (if (== (Utilities|Array|Length (LocalVariables|GetReturnedLines)) 1)
    (return (Utilities|Array|Get(acopy) (LocalVariables|GetReturnedLines)))
    (else
      (Widget|RemovefromParent (Variables|Default|GetDialogueWidget))
      (Variables|Default|SetDialogueWidget 0)
      (Variables|Default|SetLineCurrnet 0))))