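; Wolf enemy character that can walk, run, attack and drain the player's health on contact.
; Walk and Run events switch movement speed, while Attack plays an animation, then restores Animation Blueprint mode after a delay.
; Tick polls overlapping actors for the player and subtracts WolfDamage from PlayerHealth, throttled by a DoOnce that resets after a delay.
; Damage runs independently of the Attack event, and the Sphere overlap event is empty.
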(event OnComponentBeginOverlap(Sphere)
  (params (OverlappedComponent :type Primitive%20Component%20Object%20Reference) (OtherActor :type Actor%20Object%20Reference) (OtherComp :type Primitive%20Component%20Object%20Reference) (OtherBodyIndex :type Integer) (bFromSweep :type Boolean) (SweepResult :type Hit%20Result%20Structure%20%28by%20ref%29)))

(event Custom|Walk
  ;[1 1 1] Switch between walk- and run speed
  (Variables|/Script/Engine.CharacterMovementComponent|SetMaxWalkSpeed (Variables|Character|GetCharacterMovement) 2e+02))

(event Custom|Run
  ;[1 1 1] Switch between walk- and run speed
  (Variables|/Script/Engine.CharacterMovementComponent|SetMaxWalkSpeed (Variables|Character|GetCharacterMovement) 4e+02))

(event Custom|Attack
  ;[1 1 1] Attack Animation
  (Components|Animation|PlayAnimation (Variables|Character|GetMesh) "/Game/Characters/Wolf/AttackMontage.AttackMontage" false)
  (Utilities|FlowControl|Delay 1.0)
  (Components|Animation|SetAnimationMode (Variables|Character|GetMesh) "AnimationBlueprint"))

(event EventTick
  (params (DeltaSeconds :type Float%20%28single-precision%29))
  (bind _returnvalue (Game|GetPlayerCharacter 0))
  (for _array_element (Collision|GetOverlappingActors "/Game/ThirdPersonCPP/Blueprints/ThirdPersonCharacter.ThirdPersonCharacter_C" :!class /Script/Engine.Actor)
    (if (== _array_element _returnvalue)
      (bind _asthird_person_character (Utilities|Casting|CastToThirdPersonCharacter _returnvalue))
      (if (> (Variables|/Script/GGJ2019.GGJ2019Character|GetplayerHealth _asthird_person_character) 0.0)
        (Utilities|FlowControl|DoOnce false :!label _label
          (:Completed
            (Variables|/Script/GGJ2019.GGJ2019Character|SetplayerHealth _asthird_person_character (- (Variables|/Script/GGJ2019.GGJ2019Character|GetplayerHealth _asthird_person_character) (Variables|Default|GetWolfDamage)))
            (Utilities|FlowControl|Delay 1.0)
            (goto _label Reset)))))))

(fn ConstructionScript)